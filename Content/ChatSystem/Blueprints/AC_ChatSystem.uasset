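; Actor component that provides multiplayer text chat, with an on-screen chat box in selected levels.
; On BeginPlay it creates WBP_ChatBox for player controller 0 if the current level name is in its Levels list.
; SendChatMessage, meant for the server, relays the message and owner's player name through the game mode's ConnectedPlayers to each chat component.
; UpdateChatLog packs both into a chat data struct for the widget.
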(event `self.ReceiveBeginPlay`
  (bind _returnvalue (`GameplayStatics.GetCurrentLevelName` true))
  (if (`KismetArrayLibrary.Array_Contains` (`self.Levels`) _returnvalue)
    (`self.InitializeChat`)))

(event `InitializeChat`
  (bind _returnvalue (`|CreateWidget` "/Game/ChatSystem/Widgets/WBP_ChatBox.WBP_ChatBox_C" (`GameplayStatics.GetPlayerController` 0)))
  (bind _output_get (set `self.ChatBoxRef` _returnvalue))
  (`UserWidget.AddToViewport` _output_get 0))

(event `SendChatMessage`
  (params (Message :type String))
  ;[1 1 1] Send Chat From Server
  (bind _asbp_third_person_game_mode (cast `/Game/ThirdPerson/Blueprints/BP_ThirdPersonGameMode` (`GameplayStatics.GetGameMode`)))
  (for _array_element (`/Game/ThirdPerson/Blueprints/BP_ThirdPersonGameMode.ConnectedPlayers` _asbp_third_person_game_mode)
    (bind _playername (message `/Game/ChatSystem/Blueprints/BPI_Chat.GetPlayerName` (`self.GetOwner`)))
    (`self.UpdateChatLog` (`/Game/ChatSystem/Blueprints/Demo_PC.AC_ChatSystem` _array_element) _playername Message)))

(event `UpdateChatLog`
  (params (PlayerName :type String) (Messgae :type String))
  (`/Game/ChatSystem/Widgets/WBP_ChatBox.UpdateChatLog` (`self.ChatBoxRef`) (make `/Game/ChatSystem/Data/ChatDataStruct` PlayerName Messgae)))