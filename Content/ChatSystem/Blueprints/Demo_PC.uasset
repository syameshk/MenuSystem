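; Demo player controller for the chat system, carrying the ACChatSystem component and letting the player switch in and out of chat input.
; The T key runs ToggleChat, which flips the mouse cursor and swaps between Game and UI and Game Only input modes, then prints a debug message.
; Two getter functions expose the chat component and the player's name from the PlayerState.
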(event `Key|T`
  (params (Key :type "Key Structure"))
  (:`Pressed`
    (`self.ToggleChat`)
    (`KismetSystemLibrary.PrintString` "Toggle Chat")))

(event `ToggleChat`
  (bind _output_get (set `self.bShowMouseCursor` (not (`self.bShowMouseCursor`))))
  (if _output_get
    (`WidgetBlueprintLibrary.SetInputMode_GameAndUIEx` self null)
    (else
      (`WidgetBlueprintLibrary.SetInputMode_GameOnly` self))))

(fn `GetChatSystemComponent`
  (returns (ChatSystemComponent :type "/Game/ChatSystem/Blueprints/AC_ChatSystem Object Reference"))
  (return (`self.AC_ChatSystem`)))

(fn `GetPlayerName`
  (returns (PlayerName :type String))
  (return (`PlayerState.GetPlayerName` (`self.PlayerState`))))

(fn `UserConstructionScript`)