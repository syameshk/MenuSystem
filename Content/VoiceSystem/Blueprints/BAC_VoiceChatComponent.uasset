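; Voice chat component that drives an Agora engine for joining, leaving and muting a voice channel.
; It initializes the Agora engine on BeginPlay and releases it on EndPlay.
; Hardcoded keyboard events call the join, leave, mute and unmute functions directly, each printing a debug string first.
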(event `self.ReceiveBeginPlay`
  (`self.InitAgoraEngine`))

(event `Key|J`
  (params (Key :type "Key Structure"))
  (:`Pressed`
    (`KismetSystemLibrary.PrintString` "Join")
    (`self.JoinChannel`)))

(event `Key|L`
  (params (Key :type "Key Structure"))
  (:`Pressed`
    (`KismetSystemLibrary.PrintString` "Leave")
    (`self.LeaveChannel`)))

(event `Key|M`
  (params (Key :type "Key Structure"))
  (:`Pressed`
    (`KismetSystemLibrary.PrintString` "Mute")
    (`self.ToggleMute` true)))

(event `Key|U`
  (params (Key :type "Key Structure"))
  (:`Pressed`
    (`KismetSystemLibrary.PrintString` "UnmuteU")
    (`self.ToggleMute` false)))

(event `self.ReceiveEndPlay`
  (params (EndPlayReason :type "EEndPlayReason Enum" :default "Destroyed"))
  (`self.ReleaseAgoraEngine`))